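; Test game mode that keeps a registry of BP_StrafeTarget bots and respawns them when they die.
; RegisterBot stores each bot with its start transform and CanMove flag in parallel arrays, and binds to its OnBotDie event.
; The death handler spawns a replacement at the saved transform, restores CanMove and overwrites the same array slot, without binding the replacement's death event itself.
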(event `self.ReceiveBeginPlay`)

(event `CustomEvent`
  (params (Bot :type "/Game/FPS/Test/BP_StrafeTarget Object Reference"))
  (bind _returnvalue (`KismetArrayLibrary.Array_Find` (`self.Bot`) Bot))
  (if (>= _returnvalue 0)
    (remove `/Game/FPS/Test/BP_StrafeTarget.OnBotDie` Bot (delegate `CustomEvent`))
    (bind _returnvalue_2 (`|SpawnActorFromClass` "/Game/FPS/Test/BP_StrafeTarget.BP_StrafeTarget_C" (`KismetMathLibrary.MakeTransform` (.location (`|GetArrayItem` (`self.StartTransform`) _returnvalue)) (.rotation (`|GetArrayItem` (`self.StartTransform`) _returnvalue)) (.scale (`|GetArrayItem` (`self.StartTransform`) _returnvalue))) "Undefined" "MultiplyWithRoot" null null))
    (set `/Game/FPS/Test/BP_StrafeTarget.CanMove` (`|GetArrayItem` (`self.CanMove`) _returnvalue) _returnvalue_2)
    (`KismetArrayLibrary.Array_Set` (`self.Bot`) _returnvalue _returnvalue_2)))

(fn `RegisterBot`
  (params (Bot :type "Actor Object Reference"))
  (bind _asbp_strafe_target (cast `/Game/FPS/Test/BP_StrafeTarget` Bot))
  (`/Engine/EditorBlueprintResources/StandardMacros.IsValid` _asbp_strafe_target
    (:`Is Valid`
      (`KismetArrayLibrary.Array_Add` (`self.Bot`) _asbp_strafe_target)
      (`KismetArrayLibrary.Array_Add` (`self.StartTransform`) (`self.GetTransform` _asbp_strafe_target))
      (`KismetArrayLibrary.Array_Add` (`self.Start Location`) (`/Game/FPS/Test/BP_StrafeTarget.StartLocation` _asbp_strafe_target))
      (`KismetArrayLibrary.Array_Add` (`self.CanMove`) (`/Game/FPS/Test/BP_StrafeTarget.CanMove` _asbp_strafe_target))
      (add `/Game/FPS/Test/BP_StrafeTarget.OnBotDie` _asbp_strafe_target (`|CreateDelegate` :!event `CustomEvent`)))))

(fn `UserConstructionScript`)