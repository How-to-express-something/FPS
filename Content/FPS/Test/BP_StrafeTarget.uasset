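; BP_StrafeTarget is a test bot that strafes back and forth as a moving target.
; On BeginPlay the server registers it with BP_TestGameMode and stores its start location and right vector.
; While movement is enabled and it is alive, server Tick feeds movement input along that axis, reversing at HalfDistance either side of the start.
; Server_SetMove toggles movement, and the 2 key switches weapons through CombatComponent.
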(event `self.ReceiveBeginPlay`
  (if (`self.HasAuthority`)
    (bind _asbp_test_game_mode (cast `/Game/FPS/Test/BP_TestGameMode` (`GameplayStatics.GetGameMode`)))
    (`/Engine/EditorBlueprintResources/StandardMacros.IsValid` _asbp_test_game_mode
      (:`Is Valid`
        (`/Game/FPS/Test/BP_TestGameMode.RegisterBot` _asbp_test_game_mode self)
        (set `self.StartLocation` (`self.K2_GetActorLocation`))
        (set `self.StrafeAxis` (`self.GetActorRightVector`))))))

(event `self.ReceiveTick`
  (params (DeltaSeconds :type "Float (single-precision)"))
  (bind _returnvalue (`KismetMathLibrary.Dot_VectorVector` (- (`self.K2_GetActorLocation`) (`self.StartLocation`)) (`self.StrafeAxis`)))
  (if (and (`self.HasAuthority`) (`self.CanMove`))
    (if (not (`FPSHealthComponent.bDead` (`self.HealthComponent`)))
      (`|ExecutionSequence`
        (:`then_0`
          (if (>= _returnvalue (`self.HalfDistance`))
            (set `self.MoveDirection` -1.0)
            (elif (<= _returnvalue (* (`self.HalfDistance`) -1.0))
              (set `self.MoveDirection` 1.0))))
        (:`then_1`
          (`self.AddMovementInput` (`self.StrafeAxis`) (`self.MoveDirection`)))))))

(event `Key|Two`
  (params (Key :type "Key Structure"))
  (:`Pressed`
    (`FPSCombatComponent.SwitchWeapon` (`self.CombatComponent`) 1)))

(event `Server_SetMove`
  (set `self.CanMove` (not (`self.CanMove`))))

(fn `UserConstructionScript`)